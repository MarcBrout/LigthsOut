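; OpenableShelf_BP is a shelf that slides open when its ShelfEvent OnTrigger event fires.
; BeginPlay stores the starting location, and the ShelfOpening timeline's DoorCurve offsets it along world X on each update.
; Timeline event tracks play a lock sound at the shelf, then a wood bump and wind gust, with the bump placed at world origin rather than the actor.
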(event `self.ShelfEvent.OnTrigger`
  (bind _returnvalue (`self.K2_GetActorLocation`))
  (bind (_direction _doorcurve) (`Timeline|Shelf Opening`)
    (:`Update`
      (`self.K2_SetActorLocation` (+ (`KismetMathLibrary.MakeVector` _doorcurve) (`self.Shelf location`))))
    (:`CrackSound`
      (`GameplayStatics.PlaySoundAtLocation` "/Game/Audio/door-lock.door-lock" _returnvalue))
    (:`Long`
      (`GameplayStatics.PlaySoundAtLocation` "/Game/Audio/NFF-bump-wood.NFF-bump-wood" (0.0 0.0 0.0) (struct) 0.5 0.8)
      (`GameplayStatics.PlaySoundAtLocation` "/Game/Audio/NFF-wind-gust-3.NFF-wind-gust-3" _returnvalue))))

(event `self.ReceiveBeginPlay`
  (set `self.Shelf location` (`self.K2_GetActorLocation`)))

(fn `UserConstructionScript`)